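; BP_Enemy is a 2D sprite enemy for the Space Wars minigame that wanders sideways while firing continuously.
; Tick moves it at constant speed toward a random Y target through a gate, which closes on arrival until a new target is picked after a short delay.
; Fire loops on a delay, spawning flipped BP_2DProjectile actors just below it.
; Damage briefly swaps the sprite, then reduces Health and destroys the actor at zero.
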(event Custom|Fire
  (bind _returnvalue (Transformation|GetActorTransform))
  (bind (_location _rotation _scale) (Math|Transform|BreakTransform _returnvalue))
  (bind (_roll _pitch _yaw) (Math|Rotator|BreakRotator _rotation))
  (Game|SpawnActorfromClass "/Game/Assets/SpaceWarsMiniGameAssets/Blueprints/BP_2DProjectile.BP_2DProjectile_C" (Math|Transform|MakeTransform (+ _location "0,0,-15.000000") (Math|Rotator|MakeRotator (+ _roll -1.8e+02) _pitch _yaw) _scale) "Undefined" 0 0)
  (Utilities|FlowControl|Delay 0.5)
  (CallFunction|Fire))

(event Custom|Get%20New%20Target%20Location
  (bind _returnvalue (Transformation|GetActorLocation))
  (bind (_x _y _z) (Math|Vector|BreakVector _returnvalue))
  (Utilities|FlowControl|Delay 0.2)
  (bind _output_get (Variables|Default|SetTargetLocation (Math|Vector|MakeVector _x (Math|Random|RandomFloatinRange -2.5e+02 2.5e+02) _z)))
  (Utilities|FlowControl|Gate false) ; enters at Open
)

(event EventBeginPlay
  (bind _returnvalue (Transformation|GetActorLocation))
  (bind (_x _y _z) (Math|Vector|BreakVector _returnvalue))
  (CallFunction|Fire)
  (Variables|Default|SetTargetLocation (Math|Vector|MakeVector _x (Math|Random|RandomFloatinRange -2.5e+02 2.5e+02) _z)))

(event EventTick
  (params (DeltaSeconds :type Float%20%28single-precision%29))
  (Utilities|FlowControl|Gate false :!label _label
    (:Exit
      (Transformation|Teleport (Math|Interpolation|VInterptoConstant (Transformation|GetActorLocation) (stale Custom|Get%20New%20Target%20Location _output_get) (Utilities|Time|GetWorldDeltaSeconds) 1e+02) "0, 0, 0")
      (if (Utilities|Operators|EqualEqual (Transformation|GetActorLocation) (Variables|Default|GetTargetLocation) 1.0)
        (CallFunction|GetNewTargetLocation)
        (goto _label Close)))))

(event EventOnTakeDamage
  (params (damageAmount :type Float%20%28double-precision%29) (isSilentKill :type Boolean))
  (Rendering|Components|Sprite|SetSprite (Variables|Default|GetPaperSprite) "/Game/Assets/SpaceWarsMiniGameAssets/Sprites/EnemyDamage_Sprite_0.EnemyDamage_Sprite_0")
  (Utilities|FlowControl|Delay 0.05)
  (Rendering|Components|Sprite|SetSprite (Variables|Default|GetPaperSprite) "/Game/Assets/SpaceWarsMiniGameAssets/Sprites/Enemy_Sprite_0.Enemy_Sprite_0")
  (bind _output_get (Variables|Default|SetHealth (- (Variables|Default|GetHealth) damageAmount)))
  (if (<= _output_get 0.0)
    (Actor|DestroyActor)))

(fn ConstructionScript)

(fn GetIsDead
  (return false))