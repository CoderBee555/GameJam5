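; Player ship for the Space Wars minigame, a 2D flipbook pawn that moves vertically and sideways.
; Fire loops itself through a delay to auto-spawn projectiles, while damage updates the HUD and flashes a damaged flipbook.
; Death marks the server hack failed in the save and opens MainLevel.
; BeginPlay and F save position to the same "Default" slot through a different save class, then only print it.
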(event Custom|Fire
  (bind _returnvalue (Transformation|GetActorTransform))
  (bind (_location _rotation _scale) (Math|Transform|BreakTransform _returnvalue))
  (Game|SpawnActorfromClass "/Game/Assets/SpaceWarsMiniGameAssets/Blueprints/BP_2DProjectile.BP_2DProjectile_C" (Math|Transform|MakeTransform (+ _location "0,0,30.000000") _rotation _scale) "Undefined" 0 0)
  (Utilities|FlowControl|Delay 0.2)
  (CallFunction|Fire))

(event EventBeginPlay
  (CallFunction|Fire)
  (CallFunction|SaveGame)
  (CallFunction|LoadGame)
  (bind _returnvalue (UserInterface|CreateWidget "/Game/Assets/SpaceWarsMiniGameAssets/Widgets/UI_SpaceWarsHUD.UI_SpaceWarsHUD_C" 0 self))
  (bind _output_get (Variables|Default|SetUI_HUD _returnvalue))
  (UserInterface|Viewport|AddtoViewport _output_get 0))

(event EventOnTakeDamage
  (params (damageAmount :type Float%20%28double-precision%29) (isSilentKill :type Boolean))
  (Default|TakeDamage (Variables|Default|GetUI_HUD))
  (Sprite|SetFlipbook (Variables|Default|GetSprite) "/Game/Assets/SpaceWarsMiniGameAssets/Sprites/PlayerMiniGameShipDamaged1.PlayerMiniGameShipDamaged1")
  (Utilities|FlowControl|Delay 0.05)
  (Sprite|SetFlipbook (Variables|Default|GetSprite) "/Game/Assets/SpaceWarsMiniGameAssets/Sprites/PlayerAnim.PlayerAnim")
  (bind _output_get (Variables|Default|SetHealth (- (Variables|Default|GetHealth) damageAmount)))
  (if (<= _output_get 0.0)
    (bind _returnvalue (SaveGame|LoadGamefromSlot "Default"))
    (bind _asbp_save_game (Utilities|Casting|CastToBP_SaveGame _returnvalue))
    (Variables|/Game/Blueprints/SaveGame/BP_SaveGame.BP_SaveGame_C|SetisServerSuccesfullyHacked _asbp_save_game false)
    (SaveGame|SaveGametoSlot _returnvalue "Default")
    (Game|OpenLevel(byName) "MainLevel")))

(event Input|AxisEvents|InputAxisMoveRight/Left
  (params (AxisValue :type Float%20%28single-precision%29))
  (Pawn|Input|AddMovementInput "0,1.000000, 0" AxisValue false))

(event Input|AxisEvents|InputAxisMoveForward/Backward
  (params (AxisValue :type Float%20%28single-precision%29))
  (Pawn|Input|AddMovementInput "0.000000,0.000000,1.000000" AxisValue false))

(event Input|KeyboardEvents|F
  (params (Key :type Key%20Structure :default "None"))
  (:Pressed
    (CallFunction|SaveGame)
    (CallFunction|LoadGame)))

(fn ConstructionScript)

(fn SaveGame
  (bind _returnvalue (SaveGame|DoesSaveGameExist "Default"))
  (if _returnvalue
    (bind _returnvalue_2 (SaveGame|LoadGamefromSlot "Default"))
    (bind _asbp_save_game_adsa (Utilities|Casting|CastToBP_SaveGame-adsa _returnvalue_2))
    (Variables|/Game/Assets/SpaceWarsMiniGameAssets/Blueprints/BP_SaveGame-adsa.BP_SaveGame-adsa_C|SetPosition _asbp_save_game_adsa (Transformation|GetActorLocation))
    (SaveGame|SaveGametoSlot _asbp_save_game_adsa "Default")
    (else
      (bind _returnvalue_3 (SaveGame|CreateSaveGameObject "/Game/Assets/SpaceWarsMiniGameAssets/Blueprints/BP_SaveGame-adsa.BP_SaveGame-adsa_C"))
      (SaveGame|SaveGametoSlot _returnvalue_3 "Default")
      (bind _asbp_save_game_adsa_2 (Utilities|Casting|CastToBP_SaveGame-adsa _returnvalue_3))
      (Variables|/Game/Assets/SpaceWarsMiniGameAssets/Blueprints/BP_SaveGame-adsa.BP_SaveGame-adsa_C|SetPosition _asbp_save_game_adsa_2 (Transformation|GetActorLocation))
      (SaveGame|SaveGametoSlot _asbp_save_game_adsa_2 "Default"))))

(fn LoadGame
  (bind _returnvalue (SaveGame|LoadGamefromSlot "Default"))
  (bind _asbp_save_game_adsa (Utilities|Casting|CastToBP_SaveGame-adsa _returnvalue))
  (Development|PrintString (Utilities|String|ToString(Vector) (Variables|/Game/Assets/SpaceWarsMiniGameAssets/Blueprints/BP_SaveGame-adsa.BP_SaveGame-adsa_C|GetPosition _asbp_save_game_adsa))))

(fn GetIsDead
  (return false))