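; Interactable control panel that starts the "SpaceWarMiniGame" minigame when the player interacts to hack the servers.
; Entering the R trigger caches the BP_ThirdPersonCharacter, shows a Turkish "press E" prompt and registers the panel as its InteractionObject.
; A never-reset DoOnce before the cast limits this to the first overlap by any actor.
; Leaving removes the prompt and clears the InteractionObject.
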(event OnComponentBeginOverlap(r)
  (params (OverlappedComponent :type Primitive%20Component%20Object%20Reference) (OtherActor :type Actor%20Object%20Reference) (OtherComp :type Primitive%20Component%20Object%20Reference) (OtherBodyIndex :type Integer) (bFromSweep :type Boolean) (SweepResult :type Hit%20Result%20Structure%20%28by%20ref%29))
  (Utilities|FlowControl|DoOnce false
    (:Completed
      (bind _asbp_third_person_character (Utilities|Casting|CastToBP_ThirdPersonCharacter OtherActor))
      (Variables|Default|SetPlayer _asbp_third_person_character)
      (Variables|/Game/UI/UIMessage.UIMessage_C|SetMessage (Variables|/Game/ThirdPerson/Blueprints/BP_ThirdPersonCharacter.BP_ThirdPersonCharacter_C|GetUIMessage (Variables|Default|GetPlayer)) "Serverları hack'lemek için E ye basın")
      (UserInterface|Viewport|AddtoViewport (Variables|/Game/ThirdPerson/Blueprints/BP_ThirdPersonCharacter.BP_ThirdPersonCharacter_C|GetUIMessage (Variables|Default|GetPlayer)) 0)
      (Variables|/Game/ThirdPerson/Blueprints/BP_ThirdPersonCharacter.BP_ThirdPersonCharacter_C|SetInteractionObject (Variables|Default|GetPlayer) self))))

(event OnComponentEndOverlap(r)
  (params (OverlappedComponent :type Primitive%20Component%20Object%20Reference) (OtherActor :type Actor%20Object%20Reference) (OtherComp :type Primitive%20Component%20Object%20Reference) (OtherBodyIndex :type Integer))
  (bind _asbp_third_person_character (Utilities|Casting|CastToBP_ThirdPersonCharacter OtherActor))
  (Widget|RemovefromParent (Variables|/Game/ThirdPerson/Blueprints/BP_ThirdPersonCharacter.BP_ThirdPersonCharacter_C|GetUIMessage _asbp_third_person_character))
  (Variables|/Game/ThirdPerson/Blueprints/BP_ThirdPersonCharacter.BP_ThirdPersonCharacter_C|SetInteractionObject _asbp_third_person_character 0))

(event EventInteract
  (Default|StartMiniGame (Variables|Default|GetPlayer) "SpaceWarMiniGame"))

(fn ConstructionScript)