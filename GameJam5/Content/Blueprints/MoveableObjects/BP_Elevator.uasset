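; BP_Elevator is a moving platform that travels between two locations defined as offsets from its starting position.
; A BP_ThirdPersonCharacter overlapping component R opens a gate on Tick, and leaving it closes the gate, halting movement.
; While open, constant-speed interpolation moves the actor toward the other location.
; Arrival, checked by height going to the second location and by near-equality returning, flips the index and closes the gate.
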(event OnComponentBeginOverlap(r)
  (params (OverlappedComponent :type Primitive%20Component%20Object%20Reference) (OtherActor :type Actor%20Object%20Reference) (OtherComp :type Primitive%20Component%20Object%20Reference) (OtherBodyIndex :type Integer) (bFromSweep :type Boolean) (SweepResult :type Hit%20Result%20Structure%20%28by%20ref%29))
  (bind _locations (Variables|Default|GetLocations))
  (bind _locations_2 (Variables|Default|GetLocations))
  (bind _initactor_location (Variables|Default|GetInitActor%20Location))
  (bind _output (Utilities|Array|Get(acopy) _locations))
  (bind _output_2 (Utilities|Array|Get(acopy) _locations_2 1))
  (bind _returnvalue (+ _output _initactor_location))
  (bind _returnvalue_2 (+ _output_2 _initactor_location))
  (Utilities|Casting|CastToBP_ThirdPersonCharacter OtherActor)
  (Utilities|FlowControl|Gate true) ; enters at Open
)

(event OnComponentEndOverlap(r)
  (params (OverlappedComponent :type Primitive%20Component%20Object%20Reference) (OtherActor :type Actor%20Object%20Reference) (OtherComp :type Primitive%20Component%20Object%20Reference) (OtherBodyIndex :type Integer))
  (bind _locations (Variables|Default|GetLocations))
  (bind _locations_2 (Variables|Default|GetLocations))
  (bind _initactor_location (Variables|Default|GetInitActor%20Location))
  (bind _output (Utilities|Array|Get(acopy) _locations))
  (bind _output_2 (Utilities|Array|Get(acopy) _locations_2 1))
  (bind _returnvalue (+ _output _initactor_location))
  (bind _returnvalue_2 (+ _output_2 _initactor_location))
  (Utilities|Casting|CastToBP_ThirdPersonCharacter OtherActor)
  (Utilities|FlowControl|Gate true) ; enters at Close
)

(event EventBeginPlay
  (Variables|Default|SetInitActor%20Location (Transformation|GetActorLocation)))

(event EventTick
  (params (DeltaSeconds :type Float%20%28single-precision%29))
  (bind _locations (Variables|Default|GetLocations))
  (bind _locations_2 (Variables|Default|GetLocations))
  (bind _initactor_location (Variables|Default|GetInitActor%20Location))
  (bind _output (Utilities|Array|Get(acopy) _locations))
  (bind _output_2 (Utilities|Array|Get(acopy) _locations_2 1))
  (bind _returnvalue (+ _output _initactor_location))
  (bind _returnvalue_2 (+ _output_2 _initactor_location))
  (Utilities|FlowControl|Gate true :!label _label
    (:Exit
      (switch int (Variables|Default|GetCurentLocationIndex)
        (:0
          (Transformation|SetActorLocation (Math|Interpolation|VInterptoConstant (Transformation|GetActorLocation) _returnvalue_2 (Utilities|Time|GetWorldDeltaSeconds) 2e+02) false false)
          (if (>= (.Z (Math|Vector|BreakVector (Transformation|GetActorLocation))) (.Z (Math|Vector|BreakVector _returnvalue_2)))
            (Variables|Default|SetCurentLocationIndex 1)
            (goto _label Close)))
        (:1
          (Transformation|SetActorLocation (Math|Interpolation|VInterptoConstant (Transformation|GetActorLocation) _returnvalue (Utilities|Time|GetWorldDeltaSeconds) 2e+02) false false)
          (if (Utilities|Operators|EqualEqual (Transformation|GetActorLocation) _returnvalue 1.0)
            (Variables|Default|SetCurentLocationIndex 0)
            (goto _label Close)))))))

(fn ConstructionScript)